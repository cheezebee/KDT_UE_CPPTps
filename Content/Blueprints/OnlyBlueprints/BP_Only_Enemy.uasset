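; BP_Only_Enemy is an enemy Blueprint that tracks hit points and drives a state machine in response to damage.
; BeginPlay sets current HP to max and assigns the FSM reference.
; DamageProcess subtracts incoming damage, then tells the FSM to switch to one state while HP remains above zero, or another once it is depleted.
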(event EventBeginPlay
  (Variables|Default|SetFSM (Variables|Default|GetFSM))
  (Variables|Default|SetcurrHP (Variables|Default|GetmaxHP)))

(event Collision|EventActorBeginOverlap
  (params (OtherActor :type Actor%20Object%20Reference)))

(event EventTick
  (params (DeltaSeconds :type Float%20%28single-precision%29)))

(fn ConstructionScript)

(fn DamageProcess
  (params (damage :type Integer))
  (bind _output_get (Variables|Default|SetcurrHP (- (Variables|Default|GetcurrHP) damage)))
  (if (> _output_get 0)
    (Default|ChangeState (Variables|Default|GetFSM) "NewEnumerator3")
    (else
      (Default|ChangeState (Variables|Default|GetFSM) "NewEnumerator4"))))