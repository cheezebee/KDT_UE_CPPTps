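; Third-person shooter player character with Enhanced Input movement, mouse look, double jump and a walk/run speed toggle.
; It switches between a rifle and a sniper by toggling mesh visibility; sniper zoom narrows the camera FOV and shows a crosshair widget.
; Firing plays a montage section chosen by run/air state, then the rifle spawns bullet actors while the sniper line-traces from the camera to damage BP_Only_Enemy.
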(event Input|EnhancedActionEvents|EnhancedInputActionIA_Jump
  (params (ActionValue :type Boolean) (ElapsedSeconds :type Float%20%28double-precision%29) (TriggeredSeconds :type Float%20%28double-precision%29) (InputAction :type Input%20Action%20Object%20Reference :default "/Game/Input/IA_Jump.IA_Jump"))
  (:Started
    (Character|Jump)))

(event Input|EnhancedActionEvents|EnhancedInputActionIA_Fire
  (params (ActionValue :type Float%20%28double-precision%29) (ElapsedSeconds :type Float%20%28double-precision%29) (TriggeredSeconds :type Float%20%28double-precision%29) (InputAction :type Input%20Action%20Object%20Reference :default "/Game/Input/IA_Fire.IA_Fire"))
  (CallFunction|ChangeWeapon (Math|Float|Truncate ActionValue)))

(event Input|EnhancedActionEvents|EnhancedInputActionIA_MouseMove
  (params (ActionValue :type Vector%202D%20Structure) (ElapsedSeconds :type Float%20%28double-precision%29) (TriggeredSeconds :type Float%20%28double-precision%29) (InputAction :type Input%20Action%20Object%20Reference :default "/Game/Input/IA_MouseMove.IA_MouseMove"))
  (Pawn|Input|AddControllerYawInput (.x ActionValue))
  (Pawn|Input|AddControllerPitchInput (.y ActionValue)))

(event Input|EnhancedActionEvents|EnhancedInputActionIA_Move
  (params (ActionValue :type Vector%202D%20Structure) (ElapsedSeconds :type Float%20%28double-precision%29) (TriggeredSeconds :type Float%20%28double-precision%29) (InputAction :type Input%20Action%20Object%20Reference :default "/Game/Input/IA_Move.IA_Move"))
  (CallFunction|MoveAction ActionValue))

(event Input|EnhancedActionEvents|EnhancedInputActionIA_Zoom
  (params (ActionValue :type Boolean) (ElapsedSeconds :type Float%20%28double-precision%29) (TriggeredSeconds :type Float%20%28double-precision%29) (InputAction :type Input%20Action%20Object%20Reference :default "/Game/Input/IA_Zoom.IA_Zoom"))
  ;[1 1 1] 스나이퍼 모드니?
  (if (== (Variables|Default|GetCurrWeaponMode) 2)
    (CallFunction|ZoominOut ActionValue)))

(event Input|EnhancedActionEvents|EnhancedInputActionIA_RealFire
  (params (ActionValue :type Boolean) (ElapsedSeconds :type Float%20%28double-precision%29) (TriggeredSeconds :type Float%20%28double-precision%29) (InputAction :type Input%20Action%20Object%20Reference :default "/Game/Input/IA_RealFire.IA_RealFire"))
  (CallFunction|Fire))

(event Input|EnhancedActionEvents|EnhancedInputActionIA_Run
  (params (ActionValue :type Boolean) (ElapsedSeconds :type Float%20%28double-precision%29) (TriggeredSeconds :type Float%20%28double-precision%29) (InputAction :type Input%20Action%20Object%20Reference :default "/Game/Input/IA_Run.IA_Run"))
  ;[1 1 1] 걷기 / 뛰기 모드 변경
  (bind _output_get (Variables|Default|SetisRun ActionValue))
  (if _output_get
    (Variables|/Script/Engine.CharacterMovementComponent|SetMaxWalkSpeed (Variables|Character|GetCharacterMovement) 5e+02)
    (else
      (Variables|/Script/Engine.CharacterMovementComponent|SetMaxWalkSpeed (Variables|Character|GetCharacterMovement) 2e+02))))

(event EventBeginPlay
  (bind _returnvalue (Game|GetPlayerCameraManager 0))
  (Variables|/Script/Engine.CharacterMovementComponent|SetMaxWalkSpeed (Variables|Character|GetCharacterMovement) (Variables|Default|GetMoveSpeed))
  ;[1 1 1] 카메라 상/하 회전 각도 제한
  (Variables|/Script/Engine.PlayerCameraManager|SetViewPitchMin _returnvalue -6e+01)
  (Variables|/Script/Engine.PlayerCameraManager|SetViewPitchMax _returnvalue 6e+01)
  ;[1 1 1] 점프 횟수 제한
  (Variables|Default|SetJumpMaxCount 2)
  ;[1 1 1] Input Mappng Context 연결
  (Input|AddMappingContext (PlayerController|LocalPlayerSubsystems|GetEnhancedInputLocalPlayerSubsystem (Game|GetPlayerController 0)) "/Game/Input/IMC_Default.IMC_Default" 0 "(bIgnoreAllPressedKeysUntilRelease=True,bForceImmediately=False,bNotifyUserSettings=False)")
  ;[1 1 1] Sniper UI 생성
  (bind _returnvalue_2 (UserInterface|CreateWidget (Variables|Default|GetSniperWidget)))
  (Variables|Default|SetSniperUI _returnvalue_2)
  (CallFunction|ChangeWeapon (Variables|Default|GetCurrWeaponMode)))

(event Collision|EventActorBeginOverlap
  (params (OtherActor :type Actor%20Object%20Reference)))

(event EventTick
  (params (DeltaSeconds :type Float%20%28single-precision%29)))

(fn ConstructionScript)

(fn MoveAction
  (params (kyeboardInput :type Vector%202D%20Structure))
  ;[1 1 1] P= P0 + vt
  (Pawn|Input|AddMovementInput (Math|Vector|Normalize (+ (* (.x kyeboardInput) (Transformation|GetActorRightVector)) (* (.y kyeboardInput) (Transformation|GetActorForwardVector)))) 1.0 false))

(fn RotateAction
  (Transformation|SetActorRotation (Math|Rotator|MakeRotator 0.0 0.0 (Variables|Default|Getmx)))
  (Transformation|SetRelativeRotation (Variables|Default|GetSpringArm) (Math|Rotator|MakeRotator 0.0 (Variables|Default|Getmy) 0.0) false false))

(fn ChangeWeapon
  (params (weaponIdx :type Integer))
  (bind _output_get (Variables|Default|SetCurrWeaponMode weaponIdx))
  (switch int _output_get ; 1 : 라이플모드(Gun), 2 : 스나이퍼모드(Sniper)
    (:1
      (Rendering|SetVisibility (Variables|Default|GetGun) true false)
      (Rendering|SetVisibility (Variables|Default|GetSniper) false false)
      ;[1 1 1] 라이플 무기로 바꿀때, 만약에 너 Zoom 을 하고 있으면 Sniper UI 를 제거해줘
      (if (UserInterface|Viewport|IsinViewport (Variables|Default|GetSniperUI))
        (CallFunction|ZoominOut false)))
    (:2
      (Rendering|SetVisibility (Variables|Default|GetGun) false false)
      (Rendering|SetVisibility (Variables|Default|GetSniper) true false))))

(fn ZoominOut
  (params (Condition :type Boolean))
  (if Condition
    ;[1 1 1] CrossHair 붙이냐 / 떼냐
    (UserInterface|Viewport|AddtoViewport (Variables|Default|GetSniperUI) 0)
    ;[1 1 1] 확대 / 축소
    (Camera|SetFieldOfView (Variables|Default|GetCamera) 45.0)
    (else
      (Widget|RemovefromParent (Variables|Default|GetSniperUI))
      (Camera|SetFieldOfView (Variables|Default|GetCamera) 9e+01))))

(fn Fire
  (bind _gun (Variables|Default|GetGun))
  (bind _camera (Variables|Default|GetCamera))
  (Animation|Montage|MontagePlay (Components|SkeletalMesh|GetAnimInstance (Variables|Character|GetMesh)) "/Game/Blueprints/Fire_Montage.Fire_Montage" 1.0 "MontageLength" 0.0 true)
  (if (Variables|Default|GetisRun)
    (if (AI|Components|NavMovement|IsFalling (Variables|Character|GetCharacterMovement))
      (Variables|Default|SetfireMontageName "Fire1")
      (else
        (Variables|Default|SetfireMontageName "Fire2")))
    (else
      (Variables|Default|SetfireMontageName "Fire1")))
  (Ability|Animation|MontageJumptoSection (Components|SkeletalMesh|GetAnimInstance (Variables|Character|GetMesh)) (Variables|Default|GetfireMontageName) 0)
  (switch int (Variables|Default|GetCurrWeaponMode)
    (:1
      ;[1 1 1] 총알 발사
      (Game|SpawnActorfromClass "/Game/Blueprints/OnlyBlueprints/BP_Only_Bullet.BP_Only_Bullet_C" (Math|Transform|MakeTransform (Transformation|GetSocketLocation _gun "FirePos") (Transformation|GetSocketRotation _gun "FirePos") "1.000000,1.000000,1.000000") "Undefined" "MultiplyWithRoot" 0 0))
    (:2
      ;[1 1 1] LineTrace 발사( 레이저 와 같다고 보자)
      (bind (_outhit _returnvalue) (Collision|LineTraceByChannel (Transformation|GetWorldLocation _camera) (+ (Transformation|GetWorldLocation _camera) (* (Math|Vector|GetForwardVector _camera) (Math|Float|MakeLiteralFloat 5e+03))) "TraceTypeQuery1" false 0 "None"))
      (if _returnvalue
        (Effects|SpawnEmitteratLocation "/Game/MilitaryWeapSilver/FX/P_Impact_Metal_Large_01.P_Impact_Metal_Large_01" (.ImpactPoint (Collision|BreakHitResult _outhit)) (Math|Rotator|MakeRotfromX (.ImpactNormal (Collision|BreakHitResult _outhit))))
        ;;[1 1 1] 만약에 맞은놈이 Enemy 야 피격처리 해라
        (if (Utilities|Enum|Equal(Enum) (Collision|GetCollisionObjectType (.HitComponent (Collision|BreakHitResult _outhit))) "ECC_GameTraceChannel1")
          (bind _asbp_only_enemy (Utilities|Casting|CastToBP_Only_Enemy (.HitActor (Collision|BreakHitResult _outhit))))
          (Default|DamageProcess _asbp_only_enemy 1))))))